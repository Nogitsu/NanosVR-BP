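; BP_Stairs is a construction-script Blueprint that builds a stair-like row of repeated meshes.
; It assigns the chosen static mesh to an instanced static mesh component, then adds one instance per unit of the length setting.
; Each instance is spaced by the mesh's bounding box extents plus an offset, multiplied by a direction vector, so the spacing follows the mesh size.
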(fn ConstructionScript
  (bind _staticmesh (Variables|Default|GetStaticMesh))
  (bind _returnvalue (StaticMesh|GetBoundingBox _staticmesh))
  (Components|StaticMesh|SetStaticMesh (Variables|Default|GetInstancedStaticMesh) (Variables|Default|GetStaticMesh))
  (for _index (range 1 (Variables|Default|GetLenght))
    (Components|InstancedStaticMesh|AddInstance (Variables|Default|GetInstancedStaticMesh) (Math|Transform|MakeTransform (* (- _index 1) (+ (Math|Vector|VectorGetAbs (.min _returnvalue)) (Math|Vector|VectorGetAbs (.max _returnvalue)) (Variables|Default|GetOffset)) (Variables|Default|GetDirection)) "0, 0, 0" "1.000000,1.000000,1.000000") false)))