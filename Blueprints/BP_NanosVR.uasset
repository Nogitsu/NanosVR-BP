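; BP_NanosVR is a possessable VR player Blueprint that handles motion controller input.
; EnableVR turns on the HMD with floor tracking, adds the VR mapping context and possesses it.
; Enhanced Input stores touch, trigger and grip states in per-hand structs and relays axes and button presses as named events, with the right thumbstick also driving a UMG widget.
; Helper functions get and set capsule child transforms by index.
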(event Custom|EnableVR
  (bind _returnvalue (Game|GetPlayerController 0))
  (Class|HeadMountedDisplayFunctionLibrary|EnableHMD true)
  (Class|HeadMountedDisplayFunctionLibrary|SetTrackingOrigin "Floor")
  (Input|AddMappingContext (PlayerController|LocalPlayerSubsystems|GetEnhancedInputLocalPlayerSubsystem _returnvalue) "/Game/NanosVR/Input/IMC_VRControllers.IMC_VRControllers" 0 "(bIgnoreAllPressedKeysUntilRelease=True,bForceImmediately=False)")
  (Pawn|Possess _returnvalue self))

(event Custom|DisableVR
  (Class|HeadMountedDisplayFunctionLibrary|EnableHMD false))

(event Input|EnhancedActionEvents|EnhancedInputActionIA_LeftThumbTouch
  (params (ActionValue :type Boolean) (ElapsedSeconds :type Float%20%28double-precision%29) (TriggeredSeconds :type Float%20%28double-precision%29) (InputAction :type Input%20Action%20Object%20Reference :default "/Game/NanosVR/Input/Actions/IA_LeftThumbTouch.IA_LeftThumbTouch"))
  (:Triggered
    (Utilities|Struct|SetmembersinST_HandStates (Variables|Default|GetL_HandState) ActionValue :!label _label))
  (:Completed
    (goto _label)))

(event Input|EnhancedActionEvents|EnhancedInputActionIA_LeftTriggerTouch
  (params (ActionValue :type Boolean) (ElapsedSeconds :type Float%20%28double-precision%29) (TriggeredSeconds :type Float%20%28double-precision%29) (InputAction :type Input%20Action%20Object%20Reference :default "/Game/NanosVR/Input/Actions/IA_LeftTriggerTouch.IA_LeftTriggerTouch"))
  (:Triggered
    (Utilities|Struct|SetmembersinST_HandStates (Variables|Default|GetL_HandState) ActionValue :!label _label))
  (:Completed
    (goto _label)))

(event Input|EnhancedActionEvents|EnhancedInputActionIA_LeftGrip
  (params (ActionValue :type Boolean) (ElapsedSeconds :type Float%20%28double-precision%29) (TriggeredSeconds :type Float%20%28double-precision%29) (InputAction :type Input%20Action%20Object%20Reference :default "/Game/NanosVR/Input/Actions/IA_LeftGrip.IA_LeftGrip"))
  (:Triggered
    (Utilities|Struct|SetmembersinST_HandStates (Variables|Default|GetL_HandState) ActionValue :!label _label))
  (:Completed
    (goto _label)))

(event Input|EnhancedActionEvents|EnhancedInputActionIA_RightGrip
  (params (ActionValue :type Boolean) (ElapsedSeconds :type Float%20%28double-precision%29) (TriggeredSeconds :type Float%20%28double-precision%29) (InputAction :type Input%20Action%20Object%20Reference :default "/Game/NanosVR/Input/Actions/IA_RightGrip.IA_RightGrip"))
  (:Triggered
    (Utilities|Struct|SetmembersinST_HandStates (Variables|Default|GetR_HandState) ActionValue :!label _label))
  (:Completed
    (goto _label)))

(event Input|EnhancedActionEvents|EnhancedInputActionIA_LeftGripAxis
  (params (ActionValue :type Float%20%28double-precision%29) (ElapsedSeconds :type Float%20%28double-precision%29) (TriggeredSeconds :type Float%20%28double-precision%29) (InputAction :type Input%20Action%20Object%20Reference :default "/Game/NanosVR/Input/Actions/IA_LeftGripAxis.IA_LeftGripAxis"))
  (:Triggered
    (Utilities|Struct|SetmembersinST_HandStates (Variables|Default|GetL_HandState) ActionValue :!label _label)
    (Default|CallAxisEvent "LeftGrip" ActionValue 0.0))
  (:Ongoing
    (goto _label))
  (:Completed
    (goto _label)))

(event Input|EnhancedActionEvents|EnhancedInputActionIA_LeftTriggerAxis
  (params (ActionValue :type Float%20%28double-precision%29) (ElapsedSeconds :type Float%20%28double-precision%29) (TriggeredSeconds :type Float%20%28double-precision%29) (InputAction :type Input%20Action%20Object%20Reference :default "/Game/NanosVR/Input/Actions/IA_LeftTriggerAxis.IA_LeftTriggerAxis"))
  (:Triggered
    (Utilities|Struct|SetmembersinST_HandStates (Variables|Default|GetL_HandState) ActionValue :!label _label)
    (Default|CallAxisEvent "LeftTrigger" ActionValue 0.0))
  (:Ongoing
    (goto _label))
  (:Completed
    (goto _label)))

(event Input|EnhancedActionEvents|EnhancedInputActionIA_RightGripAxis
  (params (ActionValue :type Float%20%28double-precision%29) (ElapsedSeconds :type Float%20%28double-precision%29) (TriggeredSeconds :type Float%20%28double-precision%29) (InputAction :type Input%20Action%20Object%20Reference :default "/Game/NanosVR/Input/Actions/IA_RightGripAxis.IA_RightGripAxis"))
  (:Triggered
    (Utilities|Struct|SetmembersinST_HandStates (Variables|Default|GetR_HandState) ActionValue :!label _label)
    (Default|CallAxisEvent "RightGrip" ActionValue 0.0))
  (:Ongoing
    (goto _label))
  (:Completed
    (goto _label)))

(event Input|EnhancedActionEvents|EnhancedInputActionIA_RightTriggerAxis
  (params (ActionValue :type Float%20%28double-precision%29) (ElapsedSeconds :type Float%20%28double-precision%29) (TriggeredSeconds :type Float%20%28double-precision%29) (InputAction :type Input%20Action%20Object%20Reference :default "/Game/NanosVR/Input/Actions/IA_RightTriggerAxis.IA_RightTriggerAxis"))
  (:Triggered
    (Utilities|Struct|SetmembersinST_HandStates (Variables|Default|GetR_HandState) ActionValue :!label _label)
    (Default|CallAxisEvent "RightTrigger" ActionValue 0.0))
  (:Ongoing
    (goto _label))
  (:Completed
    (goto _label)))

(event Input|EnhancedActionEvents|EnhancedInputActionIA_LeftThumbstick
  (params (ActionValue :type Vector%202D%20Structure) (ElapsedSeconds :type Float%20%28double-precision%29) (TriggeredSeconds :type Float%20%28double-precision%29) (InputAction :type Input%20Action%20Object%20Reference :default "/Game/NanosVR/Input/Actions/IA_LeftThumbstick.IA_LeftThumbstick"))
  (bind (_x _y) (Math|Vector2D|BreakVector2D ActionValue))
  (:Triggered
    (Default|CallAxisEvent "LeftThumbstick" _x _y :!label _label))
  (:Completed
    (goto _label)))

(event Input|EnhancedActionEvents|EnhancedInputActionIA_RightThumbstick
  (params (ActionValue :type Vector%202D%20Structure) (ElapsedSeconds :type Float%20%28double-precision%29) (TriggeredSeconds :type Float%20%28double-precision%29) (InputAction :type Input%20Action%20Object%20Reference :default "/Game/NanosVR/Input/Actions/IA_RightThumbstick.IA_RightThumbstick"))
  (bind (_x _y) (Math|Vector2D|BreakVector2D ActionValue))
  (:Triggered
    (Default|CallAxisEvent "RightThumbstick" _x _y :!label _label)
    (bind _asumg_nanos_vr (Utilities|Casting|CastToUMG_NanosVR (UserInterface|GetWidget (Variables|Default|GetR_Widget))))
    (Default|SetJoystick _asumg_nanos_vr ActionValue))
  (:Completed
    (goto _label)))

(event Input|EnhancedActionEvents|EnhancedInputActionIA_LeftXPress
  (params (ActionValue :type Boolean) (ElapsedSeconds :type Float%20%28double-precision%29) (TriggeredSeconds :type Float%20%28double-precision%29) (InputAction :type Input%20Action%20Object%20Reference :default "/Game/NanosVR/Input/Actions/IA_LeftXPress.IA_LeftXPress"))
  (:Started
    (Default|CallBoolEvent "XButton" true))
  (:Completed
    (Default|CallBoolEvent "XButton" false)))

(event Input|EnhancedActionEvents|EnhancedInputActionIA_LeftYPress
  (params (ActionValue :type Boolean) (ElapsedSeconds :type Float%20%28double-precision%29) (TriggeredSeconds :type Float%20%28double-precision%29) (InputAction :type Input%20Action%20Object%20Reference :default "/Game/NanosVR/Input/Actions/IA_LeftYPress.IA_LeftYPress"))
  (:Started
    (Default|CallBoolEvent "YButton" true))
  (:Completed
    (Default|CallBoolEvent "YButton" false)))

(event Input|EnhancedActionEvents|EnhancedInputActionIA_LeftXTouch
  (params (ActionValue :type Boolean) (ElapsedSeconds :type Float%20%28double-precision%29) (TriggeredSeconds :type Float%20%28double-precision%29) (InputAction :type Input%20Action%20Object%20Reference :default "/Game/NanosVR/Input/Actions/IA_LeftXTouch.IA_LeftXTouch"))
  (:Triggered
    (Utilities|Struct|SetmembersinST_HandStates (Variables|Default|GetL_HandState) ActionValue :!label _label))
  (:Completed
    (goto _label)))

(event Input|EnhancedActionEvents|EnhancedInputActionIA_RightAPress
  (params (ActionValue :type Boolean) (ElapsedSeconds :type Float%20%28double-precision%29) (TriggeredSeconds :type Float%20%28double-precision%29) (InputAction :type Input%20Action%20Object%20Reference :default "/Game/NanosVR/Input/Actions/IA_RightAPress.IA_RightAPress"))
  (:Started
    (Default|CallBoolEvent "AButton" true))
  (:Completed
    (Default|CallBoolEvent "AButton" false)))

(event Input|EnhancedActionEvents|EnhancedInputActionIA_RightBPress
  (params (ActionValue :type Boolean) (ElapsedSeconds :type Float%20%28double-precision%29) (TriggeredSeconds :type Float%20%28double-precision%29) (InputAction :type Input%20Action%20Object%20Reference :default "/Game/NanosVR/Input/Actions/IA_RightBPress.IA_RightBPress"))
  (:Started
    (Default|CallBoolEvent "BButton" true))
  (:Completed
    (Default|CallBoolEvent "BButton" false)))

(event Input|EnhancedActionEvents|EnhancedInputActionIA_LeftThumbPress
  (params (ActionValue :type Boolean) (ElapsedSeconds :type Float%20%28double-precision%29) (TriggeredSeconds :type Float%20%28double-precision%29) (InputAction :type Input%20Action%20Object%20Reference :default "/Game/NanosVR/Input/Actions/IA_LeftThumbPress.IA_LeftThumbPress"))
  (:Started
    (Default|CallBoolEvent "LeftThumbstickButton" true))
  (:Completed
    (Default|CallBoolEvent "LeftThumbstickButton" false)))

(event Input|EnhancedActionEvents|EnhancedInputActionIA_RightThumbPress
  (params (ActionValue :type Boolean) (ElapsedSeconds :type Float%20%28double-precision%29) (TriggeredSeconds :type Float%20%28double-precision%29) (InputAction :type Input%20Action%20Object%20Reference :default "/Game/NanosVR/Input/Actions/IA_RightThumbPress.IA_RightThumbPress"))
  (:Started
    (Default|CallBoolEvent "RightThumbstickButton" true))
  (:Completed
    (Default|CallBoolEvent "RightThumbstickButton" false)))

(event Input|EnhancedActionEvents|EnhancedInputActionIA_LeftYTouch
  (params (ActionValue :type Boolean) (ElapsedSeconds :type Float%20%28double-precision%29) (TriggeredSeconds :type Float%20%28double-precision%29) (InputAction :type Input%20Action%20Object%20Reference :default "/Game/NanosVR/Input/Actions/IA_LeftYTouch.IA_LeftYTouch"))
  (:Triggered
    (Utilities|Struct|SetmembersinST_HandStates (Variables|Default|GetL_HandState) ActionValue :!label _label))
  (:Completed
    (goto _label)))

(event Input|EnhancedActionEvents|EnhancedInputActionIA_RightATouch
  (params (ActionValue :type Boolean) (ElapsedSeconds :type Float%20%28double-precision%29) (TriggeredSeconds :type Float%20%28double-precision%29) (InputAction :type Input%20Action%20Object%20Reference :default "/Game/NanosVR/Input/Actions/IA_RightATouch.IA_RightATouch"))
  (:Triggered
    (Utilities|Struct|SetmembersinST_HandStates (Variables|Default|GetR_HandState) ActionValue :!label _label))
  (:Completed
    (goto _label)))

(event Input|EnhancedActionEvents|EnhancedInputActionIA_RightBTouch
  (params (ActionValue :type Boolean) (ElapsedSeconds :type Float%20%28double-precision%29) (TriggeredSeconds :type Float%20%28double-precision%29) (InputAction :type Input%20Action%20Object%20Reference :default "/Game/NanosVR/Input/Actions/IA_RightBTouch.IA_RightBTouch"))
  (:Triggered
    (Utilities|Struct|SetmembersinST_HandStates (Variables|Default|GetR_HandState) ActionValue :!label _label))
  (:Completed
    (goto _label)))

(event Input|EnhancedActionEvents|EnhancedInputActionIA_RightTriggerTouch
  (params (ActionValue :type Boolean) (ElapsedSeconds :type Float%20%28double-precision%29) (TriggeredSeconds :type Float%20%28double-precision%29) (InputAction :type Input%20Action%20Object%20Reference :default "/Game/NanosVR/Input/Actions/IA_RightTriggerTouch.IA_RightTriggerTouch"))
  (:Triggered
    (Utilities|Struct|SetmembersinST_HandStates (Variables|Default|GetR_HandState) ActionValue :!label _label))
  (:Completed
    (goto _label)))

(event Input|EnhancedActionEvents|EnhancedInputActionIA_RightThumbTouch
  (params (ActionValue :type Boolean) (ElapsedSeconds :type Float%20%28double-precision%29) (TriggeredSeconds :type Float%20%28double-precision%29) (InputAction :type Input%20Action%20Object%20Reference :default "/Game/NanosVR/Input/Actions/IA_RightThumbTouch.IA_RightThumbTouch"))
  (:Triggered
    (Utilities|Struct|SetmembersinST_HandStates (Variables|Default|GetR_HandState) ActionValue :!label _label))
  (:Completed
    (goto _label)))

(event Input|EnhancedActionEvents|EnhancedInputActionIA_LeftTrigger
  (params (ActionValue :type Boolean) (ElapsedSeconds :type Float%20%28double-precision%29) (TriggeredSeconds :type Float%20%28double-precision%29) (InputAction :type Input%20Action%20Object%20Reference :default "/Game/NanosVR/Input/Actions/IA_LeftTrigger.IA_LeftTrigger"))
  (:Triggered
    (Utilities|Struct|SetmembersinST_HandStates (Variables|Default|GetL_HandState) ActionValue :!label _label))
  (:Completed
    (goto _label)))

(event Input|EnhancedActionEvents|EnhancedInputActionIA_RightTrigger
  (params (ActionValue :type Boolean) (ElapsedSeconds :type Float%20%28double-precision%29) (TriggeredSeconds :type Float%20%28double-precision%29) (InputAction :type Input%20Action%20Object%20Reference :default "/Game/NanosVR/Input/Actions/IA_RightTrigger.IA_RightTrigger"))
  (:Triggered
    (Utilities|Struct|SetmembersinST_HandStates (Variables|Default|GetR_HandState) ActionValue :!label _label))
  (:Completed
    (goto _label)))

(fn ConstructionScript)

(fn SetChildTransform
  (params (ChildIndex :type Integer) (New%20Transform%20Location :type Vector) (New%20Transform%20Rotation :type Rotator))
  (Transformation|SetRelativeTransform (Components|GetChildComponent (Variables|Collision|GetCapsuleComponent) ChildIndex) (Math|Transform|MakeTransform New%20Transform%20Location New%20Transform%20Rotation "1.000000,1.000000,1.000000") false false))

(fn GetChildTransform
  (params (ChildIndex :type Integer))
  (bind _capsulecomponent (Variables|Collision|GetCapsuleComponent))
  (bind _returnvalue (Components|GetChildComponent _capsulecomponent ChildIndex))
  (bind _returnvalue_2 (Transformation|GetRelativeTransform _returnvalue))
  (return (.location _returnvalue_2) (.rotation _returnvalue_2)))

(fn SetChildTransformOld
  (params (ChildIndex :type Integer) (NewTransform :type Transform%20%28by%20ref%29))
  (Transformation|SetRelativeTransform (Components|GetChildComponent (Variables|Collision|GetCapsuleComponent) ChildIndex) NewTransform false false))

(fn GetChildTransformOld
  (params (ChildIndex :type Integer))
  (return (Transformation|GetRelativeTransform (Components|GetChildComponent (Variables|Collision|GetCapsuleComponent) ChildIndex))))