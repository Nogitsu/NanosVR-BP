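; Construction-script actor that fills a 3D grid with instances of a chosen static mesh, sized by per-axis Repeat counts.
; Spacing comes from the mesh's bounding box plus an Offset, and every instance shares one Rotation.
; ClampArray adjusts the Materials array toward the mesh's slot count, then AssignMaterials applies each entry by index.
; ApplyCenter optionally shifts the component back by half the grid, adjusted by CenterOffset.
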(fn ConstructionScript
  (bind _repeat (Variables|Default|GetRepeat))
  (bind _staticmesh (Variables|Default|GetStaticMesh))
  (bind _returnvalue (StaticMesh|GetBoundingBox _staticmesh))
  (Components|StaticMesh|SetStaticMesh (Variables|Default|GetInstancedStaticMesh) (Variables|Default|GetStaticMesh))
  (CallFunction|ClampArray)
  (CallFunction|AssignMaterials)
  (for _index (range 1 (Math|Float|Truncate (.x _repeat)))
    (for _index_2 (range 1 (Math|Float|Truncate (.y _repeat)))
      (for _index_3 (range 1 (Math|Float|Truncate (.z _repeat)))
        (Components|InstancedStaticMesh|AddInstance (Variables|Default|GetInstancedStaticMesh) (Math|Transform|MakeTransform (* (Math|Vector|MakeVector (- _index 1) (- _index_2 1) (- _index_3 1)) (+ (Math|Vector|VectorGetAbs (.min _returnvalue)) (Math|Vector|VectorGetAbs (.max _returnvalue)) (Variables|Default|GetOffset))) (Variables|Default|GetRotation) "1.000000,1.000000,1.000000") false))))
  (CallFunction|ApplyCenter))

(fn ApplyCenter
  (bind _centeroffset (Variables|Default|GetCenterOffset))
  (bind _repeat (Variables|Default|GetRepeat))
  (bind _staticmesh (Variables|Default|GetStaticMesh))
  (bind _returnvalue (StaticMesh|GetBoundingBox _staticmesh))
  (bind _returnvalue_2 (- _repeat _centeroffset))
  (bind (_x _y _z) (Math|Vector|BreakVector _returnvalue_2))
  (if (Variables|Default|GetCenter)
    (Transformation|SetRelativeLocation (Variables|Default|GetInstancedStaticMesh) (* (+ (Math|Vector|VectorGetAbs (.min _returnvalue)) (Math|Vector|VectorGetAbs (.max _returnvalue)) (Variables|Default|GetOffset)) -0.5 (Math|Vector|MakeVector (Math|Conversions|ToFloat(Integer) (Math|Float|Floor _x)) (Math|Conversions|ToFloat(Integer) (Math|Float|Floor _y)) (Math|Conversions|ToFloat(Integer) (Math|Float|Floor _z)))) false false)))

(fn ClampArray
  (bind _materials (Variables|Default|GetMaterials))
  (bind _staticmesh (Variables|Default|GetStaticMesh))
  (bind _materials_2 (Variables|Default|GetMaterials))
  (bind _staticmesh_2 (Variables|Default|GetStaticMesh))
  (bind _returnvalue (Utilities|Array|Length _materials))
  (bind _returnvalue_2 (Utilities|Array|Length _materials_2))
  (bind _staticmaterials (Variables|/Script/Engine.StaticMesh|GetStaticMaterials _staticmesh))
  (bind _staticmaterials_2 (Variables|/Script/Engine.StaticMesh|GetStaticMaterials _staticmesh_2))
  (bind _returnvalue_3 (Utilities|Array|Length _staticmaterials))
  (bind _returnvalue_4 (Utilities|Array|Length _staticmaterials_2))
  (if (< _returnvalue_2 _returnvalue_4)
    (for _index (range (- _returnvalue_2 1) (- _returnvalue_4 1))
      (Utilities|Array|Add (Variables|Default|GetMaterials) 0))
    (elif (> _returnvalue _returnvalue_3)
      (for _index_2 (range (- _returnvalue_3 1) (- _returnvalue 1))
        (Utilities|Array|RemoveIndex (Variables|Default|GetMaterials) _index_2)))))

(fn AssignMaterials
  (for (_array_element _array_index) (Variables|Default|GetMaterials)
    (Rendering|Material|SetMaterial (Variables|Default|GetInstancedStaticMesh) _array_index _array_element)))